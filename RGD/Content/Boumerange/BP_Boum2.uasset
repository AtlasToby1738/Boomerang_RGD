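; Boomerang projectile actor that launches itself on spawn, follows a curve-driven path, then calls CallGetBack and destroys itself.
; The Mouvement timeline drives local X/Y velocity on ProjectileMovement, scaled by MaxSpeed and a range multiplier.
; BeginPlay derives that multiplier and the timeline play rate from AtomicParameters, which also scales the collider.
; TimeChange uses a FlipFlop to alternately divide and multiply play rate and MaxSpeed by the time dilation.
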(event `Move`
  (bind (_direction _x _y) (`Timeline|Mouvement` :!via `PlayFromStart`)
    (:`Update`
      (`ProjectileMovementComponent.SetVelocityInLocalSpace` (`self.ProjectileMovement`) (`KismetMathLibrary.MakeVector` (`KismetMathLibrary.Lerp` 0.0 (* (`self.MaxSpeed`) (`self.RangeMult`)) _x) (`KismetMathLibrary.Lerp` 0.0 (* (`self.MaxSpeed`) (`self.RangeMult`)) _y))))
    (:`Finished`
      (`ProjectileMovementComponent.SetVelocityInLocalSpace` (`self.ProjectileMovement`) (0.0 0.0 0.0))
      (`self.GetBack`)
      (`self.K2_DestroyActor`))))

(event `self.ReceiveBeginPlay`
  (bind (_atomicparameters_boomerangrangemult _atomicparameters_boomerangspeed _atomicparameters_hitbox_scale) (break `/Game/Boumerange/Koa/SAtomicParameters` (`self.AtomicParameters`)))
  (bind _returnvalue (* (/ 1.0 _atomicparameters_boomerangspeed) (/ (`self.MaxSpeed`) 100.0)))
  (set `self.RangeMult` (/ _atomicparameters_boomerangrangemult _returnvalue))
  (`TimelineComponent.SetPlayRate` (`self.Mouvement`) (/ 1.0 _returnvalue))
  (`SceneComponent.SetRelativeScale3D` (`self.Collider`) (`KismetMathLibrary.MakeVector` _atomicparameters_hitbox_scale _atomicparameters_hitbox_scale _atomicparameters_hitbox_scale))
  (`self.Move`))

(event `TimeChange`
  (params (TimeDilatation :type "Float (double-precision)"))
  (bind _mouvement (`self.Mouvement`))
  (bind _mouvement_2 (`self.Mouvement`))
  (`/Engine/EditorBlueprintResources/StandardMacros.FlipFlop`
    (:`A`
      (`TimelineComponent.SetPlayRate` _mouvement_2 (/ (`TimelineComponent.GetPlayRate` _mouvement_2) TimeDilatation))
      (set `self.MaxSpeed` (/ (`self.MaxSpeed`) TimeDilatation)))
    (:`B`
      (`TimelineComponent.SetPlayRate` _mouvement (* (`TimelineComponent.GetPlayRate` _mouvement) TimeDilatation))
      (set `self.MaxSpeed` (* (`self.MaxSpeed`) TimeDilatation)))))

(fn `UserConstructionScript`)