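; Boomerang projectile that flies a timeline-driven path while spinning with a looping sound, then calls GetBack and destroys itself when the path ends.
; The Mouvement timeline shapes local X/Y velocity, with range and play rate derived from AtomicParameters and MaxSpeed.
; Overlaps notify BPI_Collide actors, and anything except characters and zones bounces it by reversing path and spin.
; TimeChange toggles time dilation on movement, spin and pitch; ChangeMovementSpeed switches speed.
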(event `self.ReceiveBeginPlay`
  (bind (_atomicparameters_boomerangrangemult _atomicparameters_boomerangspeed _atomicparameters_hitbox_scale) (break `/Game/Boumerange/Koa/SAtomicParameters` (`self.AtomicParameters`)))
  (bind _returnvalue (* (/ 1.0 _atomicparameters_boomerangspeed) (/ (`self.MaxSpeed`) 100.0)))
  (bind _returnvalue_2 (`GameplayStatics.CreateSound2D` "/Game/Boumerange/Sounds/S_Floprange.S_Floprange" 1.0 1.0 0.0 null))
  (bind _output_get (set `self.BoomerangLoopingSound` _returnvalue_2))
  (`AudioComponent.Play` _output_get 0.0)
  (`self.RotationAnimation`)
  (set `self.RangeMult` (/ _atomicparameters_boomerangrangemult _returnvalue))
  (`TimelineComponent.SetPlayRate` (`self.Mouvement`) (/ 1.0 _returnvalue))
  (`SceneComponent.SetRelativeScale3D` (`self.Collider`) (`KismetMathLibrary.MakeVector` _atomicparameters_hitbox_scale _atomicparameters_hitbox_scale _atomicparameters_hitbox_scale))
  (`self.Move`))

(event `RotationAnimation`
  (`/Engine/EditorBlueprintResources/StandardMacros.FlipFlop`
    (:`A`
      (bind (_direction _rotation) (`Timeline|Rotation` :!label _label)
        (:`Update`
          (`SceneComponent.K2_SetWorldRotation` (`self.Scene`) (`KismetMathLibrary.MakeRotator` 0.0 0.0 (`KismetMathLibrary.Lerp` 0.0 360.0 _rotation)) false false))))
    (:`B`
      (goto _label :!via `Reverse`))))

(event `Move`
  (bind _boomerangloopingsound (`self.BoomerangLoopingSound`))
  (bind (_direction _x _y) (`Timeline|Mouvement` :!via `PlayFromStart` :!label _label_2)
    (:`Update`
      (`ProjectileMovementComponent.SetVelocityInLocalSpace` (`self.ProjectileMovement`) (`KismetMathLibrary.MakeVector` (`KismetMathLibrary.Lerp` 0.0 (* (`self.MaxSpeed`) (`self.RangeMult`)) _x) (`KismetMathLibrary.Lerp` 0.0 (* (`self.MaxSpeed`) (`self.RangeMult`)) _y))))
    (:`Finished`
      (`ProjectileMovementComponent.SetVelocityInLocalSpace` (`self.ProjectileMovement`) (0.0 0.0 0.0))
      (`self.GetBack`)
      (`AudioComponent.Stop` _boomerangloopingsound)
      (`ActorComponent.K2_DestroyComponent` _boomerangloopingsound)
      (`self.K2_DestroyActor`))))

(event `Reverse`
  (set `self.RangeMult` (* (`self.RangeMult`) -1.0))
  (goto _label_2 :!via `Reverse`))

(event `self.Collider.OnComponentBeginOverlap`
  (params (OverlappedComponent :type "PrimitiveComponent Object Reference") (OtherActor :type "Actor Object Reference") (OtherComp :type "PrimitiveComponent Object Reference") (OtherBodyIndex :type Integer) (bFromSweep :type Boolean) (SweepResult :type "HitResult Structure (by ref)"))
  (bind _asbpi_collide (cast `/Game/Boumerange/Character/BPI_Collide` OtherActor)
    (:`then`
      (`/Game/Boumerange/Character/BPI_Collide.Interact` _asbpi_collide self))
    (:`CastFailed`
      _))
  (`KismetSystemLibrary.IsObjectOfSoftClass` OtherActor "/Game/Boumerange/Character/BP_Character.BP_Character_C"
    (:`True`
      (`GameplayStatics.PlaySound2D` "/Game/Boumerange/Sounds/Cue/HitPlayer/SC_RobotEnd.SC_RobotEnd" 1.0 1.0 0.0 null null))
    (:`False`
      (`KismetSystemLibrary.IsObjectOfSoftClass` OtherActor "/Game/Boumerange/Zone/BP_Zone.BP_Zone_C"
        (:`False`
          (`self.Reverse`)
          (`self.RotationAnimation`)
          (`GameplayStatics.PlaySound2D` "/Game/Boumerange/Sounds/S_Bound.S_Bound" 1.0 1.0 0.0 null null))))))

(event `self.Collider.OnComponentEndOverlap`
  (params (OverlappedComponent :type "PrimitiveComponent Object Reference") (OtherActor :type "Actor Object Reference") (OtherComp :type "PrimitiveComponent Object Reference") (OtherBodyIndex :type Integer))
  (bind _asbpi_collide (cast `/Game/Boumerange/Character/BPI_Collide` OtherActor))
  (`/Game/Boumerange/Character/BPI_Collide.EndInteract` _asbpi_collide self))

(event `TimeChange`
  (params (TimeDilatation :type "Float (double-precision)") (NewPitch :type "Float (single-precision)"))
  (bind _mouvement (`self.Mouvement`))
  (bind _mouvement_2 (`self.Mouvement`))
  (bind _boomerangloopingsound (`self.BoomerangLoopingSound`))
  (bind _boomerangloopingsound_2 (`self.BoomerangLoopingSound`))
  (`/Engine/EditorBlueprintResources/StandardMacros.FlipFlop`
    (:`A`
      (`TimelineComponent.SetPlayRate` _mouvement_2 (/ (`TimelineComponent.GetPlayRate` _mouvement_2) TimeDilatation))
      (set `self.MaxSpeed` (/ (`self.MaxSpeed`) TimeDilatation))
      (`TimelineComponent.SetPlayRate` (`self.Rotation`) 0.25)
      (`/Engine/EditorBlueprintResources/StandardMacros.IsValid` _boomerangloopingsound_2
        (:`Is Valid`
          (`AudioComponent.SetPitchMultiplier` _boomerangloopingsound_2 NewPitch))))
    (:`B`
      (`TimelineComponent.SetPlayRate` _mouvement (* (`TimelineComponent.GetPlayRate` _mouvement) TimeDilatation))
      (set `self.MaxSpeed` (* (`self.MaxSpeed`) TimeDilatation))
      (`TimelineComponent.SetPlayRate` (`self.Rotation`) 1.0)
      (`/Engine/EditorBlueprintResources/StandardMacros.IsValid` _boomerangloopingsound
        (:`Is Valid`
          (`AudioComponent.SetPitchMultiplier` _boomerangloopingsound 1.0))))))

(event `ChangeMovementSpeed`
  (params (`Faster?` :type Boolean))
  (bind (_atomicparameters_boomerangrangemult _atomicparameters_boomerangspeed _atomicparameters_hitbox_scale _atomicparameters_holdtime _atomicparameters_maxthrowdistance _atomicparameters_minthrowdistance _atomicparameters_walkingspeed _atomicparameters_boomerangspeedup) (break `/Game/Boumerange/Koa/SAtomicParameters` (`self.AtomicParameters`)))
  (bind _returnvalue (* (/ 1.0 (`KismetMathLibrary.SelectFloat` _atomicparameters_boomerangspeedup _atomicparameters_boomerangspeed `Faster?`)) (/ (`self.MaxSpeed`) 100.0)))
  (set `self.RangeMult` (/ _atomicparameters_boomerangrangemult _returnvalue))
  (`TimelineComponent.SetPlayRate` (`self.Mouvement`) (/ 1.0 _returnvalue)))

(fn `UserConstructionScript`)