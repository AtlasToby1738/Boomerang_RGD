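; BP_ToolText is an actor that displays configurable text through a widget component, likely as an in-world label.
; Both the construction script and BeginPlay cast the component's widget to WBP_Text and pass the TextToShow variable to its SetUpText function.
; Running it in the construction script lets the text update in the editor as well as at runtime.
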(event `self.ReceiveBeginPlay`
  (bind _aswbp_text (cast `/Game/Boumerange/Valentin/WBP_Text` (`WidgetComponent.GetWidget` (`self.Widget`))))
  (`/Game/Boumerange/Valentin/WBP_Text.SetUpText` _aswbp_text (`self.TextToShow`)))

(fn `UserConstructionScript`
  (bind _aswbp_text (cast `/Game/Boumerange/Valentin/WBP_Text` (`WidgetComponent.GetWidget` (`self.Widget`))))
  (`/Game/Boumerange/Valentin/WBP_Text.SetUpText` _aswbp_text (`self.TextToShow`)))