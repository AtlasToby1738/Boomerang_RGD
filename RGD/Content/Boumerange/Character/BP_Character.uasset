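; Player character that moves with Enhanced Input and throws a BP_Boumerange aimed with the mouse cursor.
; Holding fire sizes an aim zone from cursor distance and boomerang parameters; release spawns the boomerang if hold time and throw range are met.
; Throwing clears CanMove; the boomerang's GetBack event restores move and fire flags and repossesses the character.
; BeginPlay also loads GameInstance parameters, shows a config widget and prepares the VFX material.
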(event `self.ReceiveBeginPlay`
  (bind _vfx (`self.VFX`))
  (`EnhancedInputSubsystemInterface.AddMappingContext` (pcsubsystem `EnhancedInputLocalPlayerSubsystem` (`GameplayStatics.GetPlayerController` 0)) "/Game/Boumerange/Input/IMC.IMC" 0 (struct))
  (set `PlayerController.bShowMouseCursor` true (`GameplayStatics.GetPlayerController` 0))
  (bind _asbp_game_instance (cast `/Game/Boumerange/Koa/BP_GameInstance` (`GameplayStatics.GetGameInstance`)))
  (`/Game/Boumerange/Koa/BP_GameInstance.LoadParameters` _asbp_game_instance)
  (bind _returnvalue (`|CreateWidget` "/Game/Widgets/WBP_ParametersConfig.WBP_ParametersConfig_C"))
  (`UserWidget.AddToViewport` _returnvalue 0)
  (`SceneComponent.SetRelativeScale3D` (`self.AimedZone(ForSize)`) (0.0 0.0 1.0))
  (bind _returnvalue_2 (`PrimitiveComponent.CreateDynamicMaterialInstance` _vfx 0 (`PrimitiveComponent.GetMaterial` _vfx 0) "None"))
  (bind _output_get (set `self.VFXMaterial` _returnvalue_2))
  (`MaterialInstanceDynamic.SetScalarParameterValue` _output_get "CircleWidth" 0.9))

(event `EnhancedInput|/Game/Boumerange/Input/AI_Move`
  (params (ActionValue :type "Vector2D Structure") (ElapsedSeconds :type "Float (double-precision)") (TriggeredSeconds :type "Float (double-precision)") (InputAction :type "InputAction Object Reference" :default "/Game/Boumerange/Input/AI_Move.AI_Move"))
  (:`Triggered`
    (`self.CanMove?`
      (:`then`
        (`self.AddMovementInput` (1.0 0.0 0.0) ActionValue_X)
        (`self.AddMovementInput` (0.0 1.0 0.0) ActionValue_Y))
      (:`else`))))

(event `EnhancedInput|/Game/Boumerange/Input/AI_Fire`
  (params (ActionValue :type Boolean) (ElapsedSeconds :type "Float (double-precision)") (TriggeredSeconds :type "Float (double-precision)") (InputAction :type "InputAction Object Reference" :default "/Game/Boumerange/Input/AI_Fire.AI_Fire"))
  (bind (_currentatomicparameters_boomerangrangemult _currentatomicparameters_boomerangspeed _currentatomicparameters_hitbox_scale _currentatomicparameters_holdtime _currentatomicparameters_maxthrowdistance _currentatomicparameters_minthrowdistance) (break `/Game/Boumerange/Koa/SAtomicParameters` (`self.CurrentAtomicParameters`)))
  (bind (_currentatomicparameters_boomerangrangemult_2 _currentatomicparameters_boomerangspeed_2 _currentatomicparameters_hitbox_scale_2 _currentatomicparameters_holdtime_2 _currentatomicparameters_maxthrowdistance_2 _currentatomicparameters_minthrowdistance_2) (break `/Game/Boumerange/Koa/SAtomicParameters` (`self.CurrentAtomicParameters`)))
  (bind (_currentatomicparameters_boomerangrangemult_3 _currentatomicparameters_boomerangspeed_3) (break `/Game/Boumerange/Koa/SAtomicParameters` (`self.CurrentAtomicParameters`)))
  (bind _hitresult (`PlayerController.GetHitResultUnderCursorByChannel` (`GameplayStatics.GetPlayerController` 0) "TraceTypeQuery1" true))
  (bind (_returnvalue_roll _returnvalue_pitch _returnvalue_yaw) (`KismetMathLibrary.BreakRotator` (`KismetMathLibrary.MakeRotFromX` (`KismetMathLibrary.GetDirectionUnitVector` (`.Location` (`GameplayStatics.BreakHitResult` _hitresult)) (`self.K2_GetActorLocation`)))))
  (bind _returnvalue (`KismetMathLibrary.Vector_Distance` (`KismetMathLibrary.MakeVector` (.x (`self.K2_GetActorLocation`)) (.y (`self.K2_GetActorLocation`))) (`KismetMathLibrary.MakeVector` (.x (`.Location` (`GameplayStatics.BreakHitResult` (`PlayerController.GetHitResultUnderCursorByChannel` (`GameplayStatics.GetPlayerController` 0) "TraceTypeQuery1" true)))) (.y (`.Location` (`GameplayStatics.BreakHitResult` (`PlayerController.GetHitResultUnderCursorByChannel` (`GameplayStatics.GetPlayerController` 0) "TraceTypeQuery1" true)))))))
  (bind _returnvalue_2 (`KismetMathLibrary.Vector_Distance` (`KismetMathLibrary.MakeVector` (.x (`self.K2_GetActorLocation`)) (.y (`self.K2_GetActorLocation`))) (`KismetMathLibrary.MakeVector` (.x (`.Location` (`GameplayStatics.BreakHitResult` _hitresult))) (.y (`.Location` (`GameplayStatics.BreakHitResult` _hitresult))))))
  (bind _returnvalue_3 (* (/ _currentatomicparameters_boomerangrangemult_3 (* (/ 1.0 _currentatomicparameters_boomerangspeed_3) (/ 1.0 (/ _returnvalue 100.0)))) 0.0767))
  (:`Ongoing`
    (if (and (> _currentatomicparameters_maxthrowdistance _returnvalue) (< _currentatomicparameters_minthrowdistance _returnvalue) (`self.CanFire?`))
      (`SceneComponent.SetRelativeScale3D` (`self.AimedZone(ForSize)`) (`KismetMathLibrary.MakeVector` _returnvalue_3 _returnvalue_3 1.0))
      (`KismetSystemLibrary.PrintString` "Hello")))
  (:`Canceled`
    (`SceneComponent.SetRelativeScale3D` (`self.AimedZone(ForSize)`) (0.0 0.0 1.0) :!label _label))
  (:`Completed`
    (if (and (> ElapsedSeconds _currentatomicparameters_holdtime_2) (> _currentatomicparameters_maxthrowdistance_2 _returnvalue_2) (< _currentatomicparameters_minthrowdistance_2 _returnvalue_2) (`self.CanFire?`))
      (set `self.CanMove?` false)
      (bind _returnvalue_4 (`|SpawnActorFromClass` "/Game/Boumerange/BP_Boumerange.BP_Boumerange_C" (`KismetMathLibrary.MakeTransform` (`self.K2_GetActorLocation`) (`KismetMathLibrary.MakeRotator` 0.0 0.0 (+ _returnvalue_yaw -90.0))) "Undefined" "MultiplyWithRoot" null _returnvalue_2 (`self.CurrentAtomicParameters`) null))
      (add `/Game/Boumerange/BP_Boumerange.GetBack` _returnvalue_4 (delegate `GetBack`))
      (else
        (goto _label)))))

(event `GetBack`
  (bind _returnvalue (`GameplayStatics.GetPlayerController` 0))
  (set `self.CanMove?` true)
  (set `self.CanFire?` true)
  (`Controller.UnPossess` _returnvalue)
  (`Controller.Possess` _returnvalue self))

(fn `UserConstructionScript`)