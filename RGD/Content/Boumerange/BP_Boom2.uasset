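; BP_Boom2 is a boomerang projectile that makes player controller 0 possess any BP_Child_Robot it overlaps.
; On BeginPlay it sizes its collider and derives timeline play rate and range multiplier from AtomicParameters and MaxSpeed, then launches.
; The Mouvement timeline's X and Y tracks drive local-space ProjectileMovement velocity to shape the flight path, and the projectile stops when the timeline finishes.
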(event `Move`
  (bind (_direction _x _y) (`Timeline|Mouvement` :!via `PlayFromStart`)
    (:`Update`
      (`ProjectileMovementComponent.SetVelocityInLocalSpace` (`self.ProjectileMovement`) (`KismetMathLibrary.MakeVector` (`KismetMathLibrary.Lerp` 0.0 (* (`self.MaxSpeed`) (`self.RangeMult`)) _x) (`KismetMathLibrary.Lerp` 0.0 (* (`self.MaxSpeed`) (`self.RangeMult`)) _y))))
    (:`Finished`
      (`ProjectileMovementComponent.SetVelocityInLocalSpace` (`self.ProjectileMovement`) (0.0 0.0 0.0)))))

(event `self.ReceiveBeginPlay`
  (bind (_atomicparameters_boomerangrangemult _atomicparameters_hitbox_scale _atomicparameters_boomerangspeed) (break `/Game/Boumerange/Koa/SAtomicParameters` (`self.AtomicParameters`)))
  (bind _returnvalue (* (/ 1.0 _atomicparameters_boomerangspeed) (/ (`self.MaxSpeed`) 100.0)))
  (`SceneComponent.SetRelativeScale3D` (`self.Collider`) (`KismetMathLibrary.MakeVector` _atomicparameters_hitbox_scale _atomicparameters_hitbox_scale _atomicparameters_hitbox_scale))
  (`TimelineComponent.SetPlayRate` (`self.Mouvement`) (/ 1.0 _returnvalue))
  (set `self.RangeMult` (/ _atomicparameters_boomerangrangemult _returnvalue))
  (`self.Move`))

(event `self.Collider.OnComponentBeginOverlap`
  (params (OverlappedComponent :type "PrimitiveComponent Object Reference") (OtherActor :type "Actor Object Reference") (OtherComp :type "PrimitiveComponent Object Reference") (OtherBodyIndex :type Integer) (bFromSweep :type Boolean) (SweepResult :type "HitResult Structure (by ref)"))
  (bind _asbp_child_robot (cast `/Game/Boumerange/Robot/BP_Child_Robot` OtherActor))
  (`Controller.Possess` (`GameplayStatics.GetPlayerController` 0) _asbp_child_robot))

(fn `UserConstructionScript`)