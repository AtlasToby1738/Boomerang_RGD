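; BP_Doors is a double sliding door, with a status LED, driven by accumulated activation values.
; Open/Close adds to a running total and, once it reaches MaxActivation, a FlipFlop alternately opens and closes the doors.
; IsOpen is never cleared, so after the first opening every call toggles regardless of the total.
; A timeline slides both panels apart from construction-cached positions or reverses, as the LED switches green or red.
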(event `Open/Close`
  (params (ActivationValue :type Integer))
  (bind _leftdoorpos (`self.LeftDoorPos`))
  (bind _rightdoorpos (`self.RightDoorPos`))
  (set `self.CurrentActivation` (+ ActivationValue (`self.CurrentActivation`)))
  (if (or (>= (`self.CurrentActivation`) (`self.MaxActivation`)) (`self.IsOpen?`))
    (`/Engine/EditorBlueprintResources/StandardMacros.FlipFlop`
      (:`A`
        (set `self.IsOpen?` true)
        (`PrimitiveComponent.SetMaterial` (`self.Led`) 0 "/Game/Boumerange/Materials/MI_Green.MI_Green")
        (bind (_direction _animation) (`Timeline|Animation` :!label _label)
          (:`Update`
            (`SceneComponent.K2_SetRelativeLocation` (`self.DoorL`) (`KismetMathLibrary.VLerp` _leftdoorpos (+ _leftdoorpos (-125.0 0.0 0.0)) _animation) false false)
            (`SceneComponent.K2_SetRelativeLocation` (`self.DoorR`) (`KismetMathLibrary.VLerp` _rightdoorpos (+ _rightdoorpos (125.0 0.0 0.0)) _animation) false false))))
      (:`B`
        (`PrimitiveComponent.SetMaterial` (`self.Led`) 0 "/Game/Boumerange/Materials/MI_Red.MI_Red")
        (goto _label :!via `Reverse`)))))

(fn `UserConstructionScript`
  (set `self.LeftDoorPos` (`SceneComponent.RelativeLocation` (`self.DoorL`)))
  (set `self.RightDoorPos` (`SceneComponent.RelativeLocation` (`self.DoorR`))))