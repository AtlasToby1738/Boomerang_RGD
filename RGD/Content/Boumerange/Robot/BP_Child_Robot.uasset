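; Child robot Blueprint that the player takes control of through an Interact event carrying a boomerang reference.
; BeginPlay runs the parent logic, then hides the PlayerSelector component.
; Interact unpossesses player 0's current pawn, possesses this robot, switches the view target to ThisCamera and stores the boomerang reference.
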(event `self.ReceiveBeginPlay`
  (`parent.ReceiveBeginPlay`)
  (`SceneComponent.SetVisibility` (`self.PlayerSelector`) false false))

(event `/Game/Boumerange/Character/BPI_Collide.Interact`
  (params (Boomrang :type "/Game/Boumerange/BP_Boumerange Object Reference"))
  (bind _returnvalue (`GameplayStatics.GetPlayerController` 0))
  (`Controller.UnPossess` _returnvalue)
  (`Controller.Possess` _returnvalue self)
  (`PlayerController.SetViewTargetWithBlend` (`GameplayStatics.GetPlayerController` 0) (`self.ThisCamera`) 0.0 "VTBlend_Linear" 0.0 false)
  (set `self.Boomerang` Boomrang))

(fn `UserConstructionScript`
  (`parent.UserConstructionScript`))